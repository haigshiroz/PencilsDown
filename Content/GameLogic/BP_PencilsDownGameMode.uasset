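; Game mode for Pencils Down, a timed classroom exam game where the player picks a squad of students who risk being caught by proctors.
; It drives title, seat selection, professor announcement, timed exam and end screens, swapping widgets and pausing or starting AI brains.
; Seat toggling respawns students as squad or regular actors within a limit.
; Scoring computes average and best grades from correctness and completion, zeroing and counting busted students.
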(event Custom|StartGamePart2_Event
  ;[0.15 0.15 0.15 0.5] Delay to allow professor to finish initial announcement
  (Utilities|FlowControl|Delay 7.0)
  (CallFunction|StartGameFunctionPart2))

(event EventBeginPlay
  (bind _returnvalue (UserInterface|CreateWidget "/Game/UI/TitleScreen_Widget.TitleScreen_Widget_C"))
  (UserInterface|Viewport|AddtoViewport _returnvalue 0)
  (Input|SetInputModeUIOnly (Game|GetPlayerController 0) _returnvalue "DoNotLock" false)
  (Utilities|FlowControl|Sequence
    (:then_0
      (bind _outactors (Actor|GetAllActorsOfClass "/Game/Characters/Proctors/BP_PD_ProctorController_Base.BP_PD_ProctorController_Base_C"))
      (for _array_element _outactors
        (AI|Logic|StopLogic (Variables|/Script/AIModule.AIController|GetBrainComponent _array_element) "")))
    (:then_1
      (bind _outactors_2 (Actor|GetAllActorsOfClass "/Game/Characters/Student/BP_PD_StudentController.BP_PD_StudentController_C"))
      (for _array_element_2 _outactors_2
        (AI|Logic|StopLogic (Variables|/Script/AIModule.AIController|GetBrainComponent _array_element_2) "")))))

(event EventTick
  (params (DeltaSeconds :type Float%20%28single-precision%29))
  (bind _output_get (Variables|Default|SetTimeRemaining (Math|Float|Max(Float) (- (Variables|Default|GetTimeRemaining) DeltaSeconds) 0.0)))
  (if (and (<= _output_get 0.0001) (Utilities|Enum|Equal(Enum) (Variables|Default|GetCurrentGameState) "NewEnumerator1"))
    (CallFunction|EndGame)))

(fn ConstructionScript)

(fn ResetGame
  (Game|OpenLevel(byObjectReference) "/Game/Maps/ClassroomMap1.ClassroomMap1" false))

(fn StartGame
  (Variables|Default|SetCurrentGameState "NewEnumerator4")
  ;[0.15 0.15 0.15 0.5] Allow professor to make announcement
  (bind _outactors (Actor|GetAllActorsOfClass "/Game/Characters/Proctors/Variants/Professor/BP_PD_Proctor_Professor_Controller.BP_PD_Proctor_Professor_Controller_C"))
  (for _array_element _outactors
    (Class|BrainComponent|RestartLogic (Variables|/Script/AIModule.AIController|GetBrainComponent _array_element))
    (AI|Logic|StartLogic (Variables|/Script/AIModule.AIController|GetBrainComponent _array_element))
    (CallFunction|StartGamePart2Event)
    (Viewport|RemoveAllWidgets)))

(fn EndGame
  (Variables|Default|SetCurrentGameState "NewEnumerator2")
  (Input|SetInputModeUIOnly (Game|GetPlayerController 0) 0 "DoNotLock" false)
  (Utilities|FlowControl|Sequence
    (:then_0
      (bind _outactors (Actor|GetAllActorsOfClass "/Game/Characters/Proctors/BP_PD_ProctorController_Base.BP_PD_ProctorController_Base_C"))
      (for _array_element _outactors
        (AI|Logic|StopLogic (Variables|/Script/AIModule.AIController|GetBrainComponent _array_element) "")))
    (:then_1
      (bind _outactors_2 (Actor|GetAllActorsOfClass "/Game/Characters/Student/BP_PD_StudentController.BP_PD_StudentController_C"))
      (for _array_element_2 _outactors_2
        (AI|Logic|StopLogic (Variables|/Script/AIModule.AIController|GetBrainComponent _array_element_2) "")))
    (:then_2
      (Viewport|RemoveAllWidgets)
      (bind _returnvalue (UserInterface|CreateWidget "/Game/UI/EndGame_Widget.EndGame_Widget_C"))
      (UserInterface|Viewport|AddtoViewport _returnvalue 0))))

(fn ScoreGame
  (bind _outactors (Actor|GetAllActorsOfClass "/Game/Characters/Student/StudentSquad/BP_PD_Student_Squad.BP_PD_Student_Squad_C"))
  (for _array_element _outactors
    (if (Variables|/Game/ExamTaking/ExamTaker.ExamTaker_C|GetBusted (Variables|/Game/Characters/Student/BP_PD_Student.BP_PD_Student_C|GetExamTaker _array_element))
      (Math|Integer|IncrementInt (LocalVariables|GetTempNumCaught))
      (else
        (LocalVariables|SetTempTotalGrade (+ (LocalVariables|GetTempTotalGrade) (* (Variables|/Game/ExamTaking/ExamTaker.ExamTaker_C|GetExamCorrectnessRate (Variables|/Game/Characters/Student/BP_PD_Student.BP_PD_Student_C|GetExamTaker _array_element)) (Variables|/Game/ExamTaking/ExamTaker.ExamTaker_C|GetExamPercentComplete (Variables|/Game/Characters/Student/BP_PD_Student.BP_PD_Student_C|GetExamTaker _array_element)))))
        (LocalVariables|SetTempMaxGrade (Math|Float|Max(Float) (LocalVariables|GetTempMaxGrade) (* (Variables|/Game/ExamTaking/ExamTaker.ExamTaker_C|GetExamCorrectnessRate (Variables|/Game/Characters/Student/BP_PD_Student.BP_PD_Student_C|GetExamTaker _array_element)) (Variables|/Game/ExamTaking/ExamTaker.ExamTaker_C|GetExamPercentComplete (Variables|/Game/Characters/Student/BP_PD_Student.BP_PD_Student_C|GetExamTaker _array_element))))))))
  (return (* (Math|Float|SafeDivide (LocalVariables|GetTempTotalGrade) (Math|Conversions|ToFloat(Integer) (Utilities|Array|Length _outactors))) 1e+02) (LocalVariables|GetTempNumCaught) (* (LocalVariables|GetTempMaxGrade) 1e+02)))

(fn SelectSeats
  (Variables|Default|SetNumberStudentsToControl 4)
  (Variables|Default|SetCurrentGameState "NewEnumerator3")
  (Input|SetInputModeGameandUI (Game|GetPlayerController 0) 0 "DoNotLock" true false)
  (Viewport|RemoveAllWidgets)
  (bind _returnvalue (UserInterface|CreateWidget "/Game/UI/StudentSelection_Widget.StudentSelection_Widget_C"))
  (UserInterface|Viewport|AddtoViewport _returnvalue 0))

(fn ToggleStudent
  (params (Student :type BP%20PD%20Student%20Object%20Reference))
  (bind _returnvalue (Utilities|GetClass Student))
  (bind _returnvalue_2 (Utilities|ClassIsChildOf _returnvalue "/Game/Characters/Student/StudentSquad/BP_PD_Student_Squad.BP_PD_Student_Squad_C"))
  (if (>= (+ (Variables|Default|GetNumberStudentsToControl) (select _returnvalue_2 1 -1)) 0)
    (Variables|Default|SetNumberStudentsToControl (+ (Variables|Default|GetNumberStudentsToControl) (select _returnvalue_2 1 -1)))
    (Game|SpawnActorfromClass (select _returnvalue_2 "/Game/Characters/Student/BP_PD_Student.BP_PD_Student_C" "/Game/Characters/Student/StudentSquad/BP_PD_Student_Squad.BP_PD_Student_Squad_C") (Transformation|GetActorTransform Student) "AlwaysSpawn" "MultiplyWithRoot" 0 0)
    (Actor|DestroyActor Student)))

(fn StartGameFunctionPart2
  (Utilities|FlowControl|Sequence
    (:then_0
      (bind _outactors (Actor|GetAllActorsOfClass "/Game/Characters/Proctors/BP_PD_ProctorController_Base.BP_PD_ProctorController_Base_C"))
      (for _array_element _outactors
        (AI|Logic|StartLogic (Variables|/Script/AIModule.AIController|GetBrainComponent _array_element))))
    (:then_1
      (bind _outactors_2 (Actor|GetAllActorsOfClass "/Game/Characters/Student/BP_PD_StudentController.BP_PD_StudentController_C"))
      (for _array_element_2 _outactors_2
        (Class|BrainComponent|RestartLogic (Variables|/Script/AIModule.AIController|GetBrainComponent _array_element_2))
        (AI|Logic|StartLogic (Variables|/Script/AIModule.AIController|GetBrainComponent _array_element_2))))
    (:then_2
      (bind _returnvalue (UserInterface|CreateWidget "/Game/UI/InGame_Widget.InGame_Widget_C"))
      (UserInterface|Viewport|AddtoViewport _returnvalue 0)
      (Variables|Default|SetTimeRemaining 3e+01)
      (Variables|Default|SetCurrentGameState "NewEnumerator1")
      (Input|SetInputModeGameandUI (Game|GetPlayerController 0) 0 "DoNotLock" true false))))
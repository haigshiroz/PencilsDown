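; BP_Controller_VariantBase is a base AI controller for character variants that steers its pawn toward a target.
; It starts brain logic on BeginPlay and stops it on UnPossess.
; Each Tick it sets the GA path component's destination to the perception component's current target position, falling back to the first player pawn's location when no target exists.
; The parent Tick call is disconnected.
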(event EventBeginPlay
  (|CallParentFunction)
  (AI|Logic|StartLogic (Variables|Default|GetBrainComponent)))

(event EventTick
  (params (DeltaSeconds :type Float%20%28single-precision%29))
  ;[0.15 0.15 0.15 0.5] Failsafe for if there's no target
  (if (Class|GAPerceptionComponent|HasTarget (Variables|Default|GetBP_PerceptionComponent))
    ;[0.15 0.15 0.15 0.5] If there is a target, use the perception component's last player location
    (Class|GAPathComponent|SetDestination (Variables|Default|GetGAPathComponent) (.Position (Utilities|Struct|BreakTargetState (.TargetStateOut (Class|GAPerceptionComponent|GetCurrentTargetState (Variables|Default|GetBP_PerceptionComponent))))))
    (else
      (Class|GAPathComponent|SetDestination (Variables|Default|GetGAPathComponent) (Transformation|GetActorLocation (Game|Player|GetPlayerPawn 0))))))

(event EventUnPossess
  (params (UnpossessedPawn :type Pawn%20Object%20Reference))
  (AI|Logic|StopLogic (Variables|Default|GetBrainComponent) ""))

(fn ConstructionScript
  (|CallParentFunction))
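; Vitality component in the AI character folder that tracks health, shield and death.
; Damage drains the shield; a hit exceeding it zeroes the shield first, so the full damage, not just overflow, comes off HP.
; Shield overwrites the current amount, which Tick decays by a fixed step per frame, independent of delta time.
; Depleted HP or Kill runs ExecuteDeath, which sets IsDead and calls Death.
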(event Custom|Damage
  (params (Location :type Vector) (Vector :type Vector) (DamageAmount :type Float%20%28double-precision%29))
  ;[0.15 0.15 0.15 0.5] If remaining shield < 0, then take from health and set shield to 0.
  ; Else, set shield to remaining shield amount
  (if (< (- (Variables|Default|GetCurrentShieldAmount) DamageAmount) 0.0)
    (Variables|Default|SetCurrentShieldAmount 0.0)
    (bind _output_get (Variables|Default|SetHP (+ (- (Variables|Default|GetCurrentShieldAmount) DamageAmount) (Variables|Default|GetHP))))
    ;[0.15 0.15 0.15 0.5] If remaining health is <= 0, execute death
    (if (<= _output_get 0.0)
      (CallFunction|ExecuteDeath))
    (else
      (Variables|Default|SetCurrentShieldAmount (- (Variables|Default|GetCurrentShieldAmount) DamageAmount)))))

(event Custom|ExecuteDeath
  (Variables|Default|SetIsDead true)
  (Default|CallDeath))

(event Custom|Kill
  (Variables|Default|SetHP 0.0)
  (CallFunction|ExecuteDeath))

(event Custom|Shield
  (params (Shield%20Amount :type Float%20%28double-precision%29))
  (Variables|Default|SetCurrentShieldAmount Shield%20Amount))

(event EventBeginPlay
  (Variables|Default|SetHP (Variables|Default|GetMaxHP)))

(event EventTick
  (params (DeltaSeconds :type Float%20%28single-precision%29))
  (Variables|Default|SetCurrentShieldAmount (Math|Float|Max(Float) (- (Variables|Default|GetCurrentShieldAmount) 1.0) 0.0)))
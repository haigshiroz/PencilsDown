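; AI controller for the Soldier enemy variant that starts its behavior tree and manages awareness of the player.
; On possess it runs BehaviorTree_Soldier.
; On any perception update, it looks up player pawn 0's target GUID in the perception component's TargetMap.
; If an entry exists, it sets Awareness straight to full and writes the struct back to the map, without inspecting the stimulus.
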(event OnPerceptionUpdated(AIPerception)
  (params (UpdatedActors :type Array%20of%20Actor%20Object%20References))
  ;[0.15 0.15 0.15 0.5] Get the Target View
  (bind _asbp_player_character (Utilities|Casting|CastToBP_PlayerCharacter (Game|Player|GetPlayerPawn 0)))
  (if (.ReturnValue (Utilities|Map|Find (Variables|/Script/GameAI.GAPerceptionComponent|GetTargetMap (Variables|Default|GetBP_PerceptionComponent)) (Variables|/Script/GameAI.GATargetComponent|GetTargetGuid (Variables|/Game/Characters/Player/BP_PlayerCharacter.BP_PlayerCharacter_C|GetGATarget _asbp_player_character))))
    (bind _structout (Utilities|Struct|SetmembersinTargetView (.Value (Utilities|Map|Find (Variables|/Script/GameAI.GAPerceptionComponent|GetTargetMap (Variables|Default|GetBP_PerceptionComponent)) (Variables|/Script/GameAI.GATargetComponent|GetTargetGuid (Variables|/Game/Characters/Player/BP_PlayerCharacter.BP_PlayerCharacter_C|GetGATarget _asbp_player_character)))) 1.0)) ; Set the awareness to 1
    ;[0.15 0.15 0.15 0.5] Re-add the component to the map
    (Utilities|Map|Add (Variables|/Script/GameAI.GAPerceptionComponent|GetTargetMap (Variables|Default|GetBP_PerceptionComponent)) (Variables|/Script/GameAI.GATargetComponent|GetTargetGuid (Variables|/Game/Characters/Player/BP_PlayerCharacter.BP_PlayerCharacter_C|GetGATarget _asbp_player_character)) _structout)))

(event EventBeginPlay
  (|CallParentFunction) ; This node is disabled and will not be called.\nDrag off pins to build functionality.
)

(event EventTick
  (params (DeltaSeconds :type Float%20%28single-precision%29))
  (|CallParentFunction DeltaSeconds) ; This node is disabled and will not be called.\nDrag off pins to build functionality.
)

(event EventPossess
  (params (PossessedPawn :type Pawn%20Object%20Reference))
  (AI|RunBehaviorTree "/Game/Characters/AICharacter/Variants/Soldier/BehaviorTree_Soldier.BehaviorTree_Soldier"))

(fn ConstructionScript
  (|CallParentFunction))
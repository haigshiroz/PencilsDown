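; Clickable squad student actor for the exam cheating game, extending a parent student with exam-progress and cheating-perception widgets.
; BeginPlay binds the widgets to its ExamTaker and GATarget components.
; A click either toggles the student through the game mode or, depending on game state and student status, updates status and opens an actions widget.
; That widget enables peek-cheating only with nearby students; clicks also print debug grid coordinates outside toggle mode.
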(event Collision|EventActorBeginOverlap
  (params (OtherActor :type Actor%20Object%20Reference)))

(event MouseInput|EventActorOnClicked
  (params (ButtonPressed :type Key%20Structure :default "None"))
  (bind _asbp_pencils_down_game_mode (Utilities|Casting|CastToBP_PencilsDownGameMode (Game|GetGameMode)))
  (if (Utilities|Enum|Equal(Enum) (Variables|/Game/GameLogic/BP_PencilsDownGameMode.BP_PencilsDownGameMode_C|GetCurrentGameState _asbp_pencils_down_game_mode) "NewEnumerator3")
    (Default|ToggleStudent _asbp_pencils_down_game_mode self)
    (else
      (CallFunction|DebugDisplayCellRefCoords)
      (Development|PrintString "Hello")
      (if (Utilities|Enum|Equal(Enum) (Variables|Default|GetStudentStatus) "NewEnumerator0")
        (CallFunction|UpdateStudentStatus "NewEnumerator2")
        (CallFunction|DisplayStudentActions)))))

(event EventBeginPlay
  (|CallParentFunction)
  (bind _asexam_progress_widget (Utilities|Casting|CastToExamProgressWidget (UserInterface|GetUserWidgetObject (Variables|Default|GetExamProgressWidget))))
  (Variables|/Game/UI/ExamProgressWidget.ExamProgressWidget_C|SetExamTaker _asexam_progress_widget (Variables|Default|GetExamTaker))
  (bind _ascheating_perception_widget (Utilities|Casting|CastToCheatingPerceptionWidget (UserInterface|GetUserWidgetObject (Variables|Default|GetCheatingPerceptionProgressWidget))))
  (Variables|/Game/UI/CheatingPerceptionWidget.CheatingPerceptionWidget_C|SetTargetComponent _ascheating_perception_widget (Variables|Default|GetGATarget)))

(fn ConstructionScript)

(fn DisplayStudentActions
  (bind _returnvalue (UserInterface|CreateWidget "/Game/UI/StudentActionsWidget.StudentActionsWidget_C" (Game|GetPlayerController 0) self))
  (UserInterface|Viewport|AddtoViewport _returnvalue 0)
  ;[0.15 0.15 0.15 0.5] If the studnet has no neighbors, they can't peak off anyone
  (bind _neighborstudents (CallFunction|GetNearbyStudents 2.5e+02))
  (Widget|SetIsEnabled (Variables|/Game/UI/StudentActionsWidget.StudentActionsWidget_C|GetButton_CheatPeek _returnvalue) (not (Utilities|Array|IsEmpty _neighborstudents)))
  (Class|Widget|SetToolTipText (Variables|/Game/UI/StudentActionsWidget.StudentActionsWidget_C|GetButton_CheatPeek _returnvalue) (Utilities|Text|MakeLiteralText "No neighbors to peek from")))

(fn DebugDisplayCellRefCoords
  (bind _outactors (Actor|GetAllActorsOfClass "/Game/Grid/BP_GridActor.BP_GridActor_C"))
  (Development|PrintString (Utilities|String|BuildString(Integer) "" (Utilities|String|BuildString(Integer) "" "(" (.X (Utilities|Struct|BreakCellRef (Class|GAGridActor|GetCellRef (Utilities|Array|Get(acopy) _outactors) (Transformation|GetActorLocation) false))) ", ") (.Y (Utilities|Struct|BreakCellRef (Class|GAGridActor|GetCellRef (Utilities|Array|Get(acopy) _outactors) (Transformation|GetActorLocation) false))) ")")))
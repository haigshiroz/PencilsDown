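; BP_PD_Student is a clickable student actor that can raise and lower its hand, shown by swapping the material on its static mesh.
; Clicking it prints a greeting, raises the hand, then prints the grid cell of its location from the first BP_GridActor found.
; LowerHand restores the screen material but is not called here.
; BeginPlay turns off occupancy map debugging on GATarget.
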(event Collision|EventActorBeginOverlap
  (params (OtherActor :type Actor%20Object%20Reference)))

(event EventTick
  (params (DeltaSeconds :type Float%20%28single-precision%29)))

(event MouseInput|EventActorOnClicked
  (params (ButtonPressed :type Key%20Structure :default "None"))
  (Development|PrintString "Hello")
  (CallFunction|RaiseHand)
  (bind _outactors (Actor|GetAllActorsOfClass "/Game/Grid/BP_GridActor.BP_GridActor_C"))
  (Development|PrintString (Utilities|String|BuildString(Integer) "" (Utilities|String|BuildString(Integer) "" "(" (.X (Utilities|Struct|BreakCellRef (Class|GAGridActor|GetCellRef (Utilities|Array|Get(acopy) _outactors) (Transformation|GetActorLocation) false))) ", ") (.Y (Utilities|Struct|BreakCellRef (Class|GAGridActor|GetCellRef (Utilities|Array|Get(acopy) _outactors) (Transformation|GetActorLocation) false))) ")")))

(event EventBeginPlay
  (Variables|/Script/GameAI.GATargetComponent|SetbDebugOccupancyMap (Variables|Default|GetGATarget) false))

(fn ConstructionScript)

(fn RaiseHand
  (Variables|Default|SetHandRaised true)
  (Rendering|Material|SetMaterial (Variables|Default|GetStaticMesh) 0 "/Game/Characters/AICharacter/Materials/Eyeball.Eyeball"))

(fn LowerHand
  (Variables|Default|SetHandRaised false)
  (Rendering|Material|SetMaterial (Variables|Default|GetStaticMesh) 0 "/Engine/EngineMaterials/ScreenMaterial.ScreenMaterial"))
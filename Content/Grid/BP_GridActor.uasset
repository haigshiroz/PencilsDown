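; BP_GridActor is a grid actor that refreshes nav-derived data and its debug and proctor-vision visuals.
; On BeginPlay and every Tick it calls refreshes for the nav data, the debug mesh and texture, and the proctor-vision mesh and texture.
; The debug texture highlights the Destination, and BeginPlay makes the proctor-vision mesh visible.
; The refresh logic itself is defined outside these graphs.
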(event EventBeginPlay
  (Class|GAGridActor|RefreshDatafromNav)
  (Class|GAGridActor|RefreshDebugMesh)
  (Class|GAGridActor|RefreshDebugTexture (Variables|Default|GetDestination) true)
  (Class|GAGridActor|RefreshProctorVisionMesh)
  (Class|GAGridActor|RefreshProctorVisionTexture)
  (Rendering|SetVisibility (Variables|Default|GetProctorVisionMeshComponent) true false))

(event Collision|EventActorBeginOverlap
  (params (OtherActor :type Actor%20Object%20Reference)))

(event EventTick
  (params (DeltaSeconds :type Float%20%28single-precision%29))
  (Class|GAGridActor|RefreshProctorVisionMesh)
  (Class|GAGridActor|RefreshProctorVisionTexture)
  (Class|GAGridActor|RefreshDatafromNav)
  (Class|GAGridActor|RefreshDebugMesh)
  (Class|GAGridActor|RefreshDebugTexture (Variables|Default|GetDestination) true))

(fn ConstructionScript)